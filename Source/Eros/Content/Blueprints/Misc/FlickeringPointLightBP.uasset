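; Point light Blueprint that flickers by toggling its visibility at random intervals.
; A non-looping timer, started on BeginPlay, fires Flicker after a random delay between the min and max flicker times, then re-arms with a new one.
; Each flicker also sets intensity by mapping the delay just elapsed onto the brightness range, so longer waits give brighter values.
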(event Custom|Flicker
  ;[1 1 1] Flicker event - toggle visibility
  (Rendering|ToggleVisibility (Variables|Default|GetPointLightComponent) true)
  ;[1 1 1] Update the light intensity
  (Rendering|Components|Light|SetIntensity (Variables|Default|GetPointLightComponent) (+ (* (/ (- (Variables|Default|GetFlickerTime) (Variables|Flicker|GetMinFlickerTime)) (- (Variables|Flicker|GetMaxFlickerTime) (Variables|Flicker|GetMinFlickerTime))) (- (Variables|Flicker|GetMaxLightBrightness) (Variables|Flicker|GetMinLightBrightness))) (Variables|Flicker|GetMinLightBrightness)))
  ;[1 1 1] Set flicker event with random time
  (bind _output_get (Variables|Default|SetFlickerTime (Math|Random|RandomFloatinRangefromStream (Variables|Flicker|GetMinFlickerTime) (Variables|Flicker|GetMaxFlickerTime) (Math|Random|MakeRandomStream (Math|Random|RandomInteger 100000)))))
  (Utilities|Time|SetTimerbyEvent (delegate Custom|Flicker) _output_get))

(event EventBeginPlay
  ;[1 1 1] Set flicker event with random time
  (bind _output_get (Variables|Default|SetFlickerTime (Math|Random|RandomFloatinRangefromStream (Variables|Flicker|GetMinFlickerTime) (Variables|Flicker|GetMaxFlickerTime) (Math|Random|MakeRandomStream (Math|Random|RandomInteger 100000)))))
  (Utilities|Time|SetTimerbyEvent (delegate Custom|Flicker) _output_get))

(fn ConstructionScript)