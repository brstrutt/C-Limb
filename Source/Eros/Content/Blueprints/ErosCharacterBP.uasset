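; Player character Blueprint for Eros that manages the HUD, pause menu and prosthetic tutorial popups.
; BeginPlay creates the HUD and binds prosthetic-swap and controller input-change events, so HUD visibility follows the input state.
; Swapping prosthetics shows that prosthetic's help widget when tutorials are enabled; Start opens the pause menu when input is enabled.
; Both pause the game and hide the HUD; Tick carries a leftover debug print.
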(event Custom|ProstheticSwapped_Event
  (params (PlayerCharacter :type Eros%20Character%20Object%20Reference) (NewProsthetic :type Prosthetic%20Object%20Reference))
  (bind _returnvalue (Game|GetPlayerController 0))
  ;[1 1 1] Show Prosthetic Tutorials
  (bind _aseros_controller (Utilities|Casting|CastToErosController (Pawn|GetController PlayerCharacter)))
  (if (Class|ErosController|GetShowProstheticTutorials _aseros_controller)
    (bind _returnvalue_2 (Class|Prosthetic|GetHelpWidget NewProsthetic))
    (bind _returnvalue_3 (UserInterface|CreateWidget _returnvalue_2))
    (Utilities|IsValid _returnvalue_3
      (:Is%20Valid
        (UserInterface|Viewport|AddtoViewport _returnvalue_3 0)
        (Widget|SetKeyboardFocus _returnvalue_3)
        (Input|SetInputModeUIOnly _returnvalue _returnvalue_3 "LockAlways")
        (Variables|/Script/Engine.PlayerController|SetbShowMouseCursor _returnvalue false)
        (Game|SetGamePaused true)
        (Widget|SetVisibility (Variables|Default|GetHUD) "Hidden")))))

(event Custom|HideHUD
  (params (NewState :type Boolean))
  (bind _hud (Variables|Default|GetHUD))
  (if NewState
    (Widget|SetVisibility _hud "Visible")
    (else
      (Widget|SetVisibility _hud "Hidden"))))

(event EventBeginPlay
  ;[1 1 1] HUD
  (bind _returnvalue (UserInterface|CreateWidget "/Game/Blueprints/UI/Menus/HUDBP.HUDBP_C"))
  (Variables|Default|SetHUD _returnvalue)
  (UserInterface|Viewport|AddtoViewport _returnvalue 0)
  ;[1 1 1] Show Prosthetic Tutorials
  (EventDispatchers|BindEventtoOnProstheticSwapped (delegate Custom|ProstheticSwapped_Event))
  (bind _aseros_controller (Utilities|Casting|CastToErosController (Pawn|GetController)))
  (EventDispatchers|UnbindallEventsfromOnInputChanged _aseros_controller)
  (EventDispatchers|AssignOnInputChanged _aseros_controller (delegate Custom|HideHUD)))

(event EventTick
  (params (DeltaSeconds :type Float%20%28single-precision%29))
  (Development|PrintString "Hello"))

(event EventDestroyed
  (Widget|RemovefromParent (Variables|Default|GetHUD)))

(event Input|ActionEvents|InputActionStartButton
  (params (Key :type Key%20Structure :default "AnyKey"))
  (:Pressed
    (bind _aseros_controller (Utilities|Casting|CastToErosController (Game|GetPlayerController 0)))
    (if (Class|ErosController|GetInputEnabled _aseros_controller)
      (bind _returnvalue (UserInterface|CreateWidget "/Game/Blueprints/UI/Menus/PauseMenuBP.PauseMenuBP_C" _aseros_controller))
      (UserInterface|Viewport|AddtoViewport _returnvalue 0)
      (Input|SetInputModeUIOnly _aseros_controller (Variables|/Game/Blueprints/UI/Menus/PauseMenuBP.PauseMenuBP_C|GetResume _returnvalue) "DoNotLock")
      (Game|SetGamePaused true)
      (Widget|SetVisibility (Variables|Default|GetHUD) "Hidden"))))

(fn ConstructionScript)

(fn SpawnHUD)